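; Destructible lighthouse that loses health when struck by a projectile and awards the player points when broken.
; On Hit it matches the other actor against all Projectile actors, prints a debug "HIT" and, if destructible, subtracts damage.
; When health equals exactly zero, it fractures the Lighthouse component with radius damage at the impact point.
; It then adds points through the player's BirdCharacterBlueprint and sets a short lifespan to remove itself.
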(event EventHit
  (params (MyComp :type Primitive%20Component%20Object%20Reference) (Other :type Actor%20Object%20Reference) (OtherComp :type Primitive%20Component%20Object%20Reference) (bSelfMoved :type Boolean) (HitLocation :type Vector :default "0, 0, 0") (HitNormal :type Vector :default "0, 0, 0") (NormalImpulse :type Vector :default "0, 0, 0") (Hit :type Hit%20Result%20Structure%20%28by%20ref%29))
  (bind _outactors (Actor|GetAllActorsOfClass "/Game/Blueprints/Projectile.Projectile_C"))
  (bind _array_element (Utilities|Array|ForEachLoopwithBreak _outactors)
    (:LoopBody
      _)
    (:Completed
      _))
  (if (== Other _array_element)
    (Rendering|Debug|DrawDebugString HitLocation "HIT" 0 "(R=0.000000,G=0.000000,B=0.000000,A=1.000000)" 3.0)
    (if (Variables|Default|GetCanBeDestoryed)
      (Variables|Default|SetHealth (- (Variables|Default|GetHealth) (Variables|Default|GetDamage)))
      (Variables|Default|SetIsHealthZero (== (Variables|Default|GetHealth) 0))
      (if (Variables|Default|GetIsHealthZero)
        (Class|DestructibleComponent|ApplyRadiusDamage (Variables|Default|GetLighthouse) 4.0 HitLocation 1e+02 5e+03 false)
        (bind _asbirdcharacterblueprint_c (Utilities|Casting|CastToBirdCharacterBlueprint (Game|Player|GetPlayerPawn 0)))
        (Variables|/Game/Blueprints/BirdCharacterBlueprint.BirdCharacterBlueprint_C|SetPointsAdded _asbirdcharacterblueprint_c (Variables|Default|GetPoints))
        (Default|AddPoints _asbirdcharacterblueprint_c)
        (Actor|SetLifeSpan 6.0)))))

(fn ConstructionScript)