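; Score Blueprint that keeps a running point total, with a reference to the bird character of an assigned player.
; On BeginPlay it casts the AssignedPlayer's character to BirdCharacterBlueprint and stores it, though nothing else here uses that reference.
; AddPoints calls GetScore, which despite its name increases Score by PointsAdded on every call before returning it.
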(event Custom|AddPoints
  (CallFunction|GetScore))

(event EventBeginPlay
  (bind _asbirdcharacterblueprint_c (Utilities|Casting|CastToBirdCharacterBlueprint (Game|GetPlayerCharacter (Variables|Default|GetAssignedPlayer))))
  (Variables|Default|SetPlayerCharacter _asbirdcharacterblueprint_c))

(fn ConstructionScript)

(fn GetScore
  (Variables|Default|SetScore (+ (Variables|Default|GetScore) (Variables|Default|GetPointsAdded)))
  (return (Variables|Default|GetScore)))