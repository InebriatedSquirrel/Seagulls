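; HUD for the bird game, drawing the minimap, altitude, poop ammo with meter, current mission and trophies every frame in DrawHUD.
; Player stats come from BirdCharacterBlueprint, and altitude is derived from pawn height.
; A nonzero Countdown makes Tick start a looping one-second TimerTicks timer, which is never explicitly cleared.
; The top-center readout shows that countdown while active, otherwise the score if ScoreActivated is set.
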(event EventDrawHUD
  (params (SizeX :type Integer) (SizeY :type Integer))
  (bind _returnvalue (Game|Player|GetOwningPlayerController))
  (bind _returnvalue_2 (Game|Player|GetPlayerPawn 0))
  (bind _myfont (Variables|Default|GetmyFont))
  (bind _fontcolor (Variables|Default|GetFontColor))
  (bind _sizex (HUD|GetViewportSize _returnvalue))
  (bind _returnvalue_3 (Math|Conversions|ToFloat(Integer) _sizex))
  (bind _returnvalue_4 (/ _returnvalue_3 2.0))
  (Canvas|DrawMaterial "/Game/UI/HUD/Minimap_Cutout.Minimap_Cutout" (- (- (Math|Conversions|ToFloat(Integer) SizeX) 5e+01) 206.0) (- (- (- (- (- (- (Math|Conversions|ToFloat(Integer) SizeY) 5e+01) 5e+01) 5e+01) 5e+01) 5e+01) 6.0) 256.0 256.0 0.0 0.0 1.0 1.0)
  (HUD|DrawText (Utilities|String|Append "Altitude: " (Utilities|String|ToString(Float) (/ (- (.Z (Math|Vector|BreakVector (Transformation|GetActorLocation _returnvalue_2))) 10937.2) 1e+02))) _fontcolor 1e+01 0.0 _myfont 1.0 false)
  (bind _asbirdcharacterblueprint_c (Utilities|Casting|CastToBirdCharacterBlueprint _returnvalue_2))
  (HUD|DrawText (Utilities|String|Append "Poop Ammo: " (Utilities|String|ToString(Integer) (Variables|/Game/Blueprints/BirdCharacterBlueprint.BirdCharacterBlueprint_C|GetAmmo _asbirdcharacterblueprint_c))) _fontcolor 1e+01 25.0 _myfont 1.0 false)
  ;[1 1 1] Poop Meters
  (if (== (Variables|/Game/Blueprints/BirdCharacterBlueprint.BirdCharacterBlueprint_C|GetAmmo _asbirdcharacterblueprint_c) 5)
    (Class|HUD|DrawMaterialSimple "/Game/UI/HUD/Mask_AmmoMeter_1_Mat.Mask_AmmoMeter_1_Mat" 0.0 0.0 5e+01 5e+01 1.0 false)
    (elif (== (Variables|/Game/Blueprints/BirdCharacterBlueprint.BirdCharacterBlueprint_C|GetAmmo _asbirdcharacterblueprint_c) 4)
      (Class|HUD|DrawMaterialSimple "/Game/UI/HUD/Mask_AmmoMeter_2_Mat.Mask_AmmoMeter_2_Mat" 0.0 0.0 5e+01 5e+01 1.0 false)
      (elif (== (Variables|/Game/Blueprints/BirdCharacterBlueprint.BirdCharacterBlueprint_C|GetAmmo _asbirdcharacterblueprint_c) 3)
        (Class|HUD|DrawMaterialSimple "/Game/UI/HUD/Mask_AmmoMeter_3_Mat.Mask_AmmoMeter_3_Mat" 0.0 0.0 5e+01 5e+01 1.0 false)
        (elif (== (Variables|/Game/Blueprints/BirdCharacterBlueprint.BirdCharacterBlueprint_C|GetAmmo _asbirdcharacterblueprint_c) 2)
          (Class|HUD|DrawMaterialSimple "/Game/UI/HUD/Mask_AmmoMeter_4_Mat.Mask_AmmoMeter_4_Mat" 0.0 0.0 5e+01 5e+01 1.0 false)
          (elif (== (Variables|/Game/Blueprints/BirdCharacterBlueprint.BirdCharacterBlueprint_C|GetAmmo _asbirdcharacterblueprint_c) 1)
            (Class|HUD|DrawMaterialSimple "/Game/UI/HUD/Mask_AmmoMeter_5_Mat.Mask_AmmoMeter_5_Mat" 0.0 0.0 5e+01 5e+01 1.0 false))))))
  (HUD|DrawText (Utilities|String|Append "Current Mission: " (Variables|/Game/Blueprints/BirdCharacterBlueprint.BirdCharacterBlueprint_C|GetMissionText _asbirdcharacterblueprint_c)) _fontcolor 1e+01 5e+01 _myfont 1.0 false)
  (HUD|DrawText (Utilities|String|Append "Trophies: " (Utilities|String|ToString(Integer) (Variables|/Game/Blueprints/BirdCharacterBlueprint.BirdCharacterBlueprint_C|GetTrophiesCollected _asbirdcharacterblueprint_c))) _fontcolor 1e+01 75.0 _myfont 1.0 false)
  (if (Variables|Default|GetTimerActivated)
    (HUD|DrawText (Utilities|String|Append "TIMER:  " (Utilities|String|ToString(Float) (Variables|Default|GetCountdown))) _fontcolor _returnvalue_4 1e+01 _myfont 1.0 false)
    (elif (Variables|Default|GetScoreActivated)
      (bind _asbirdcharacterblueprint_c_2 (Utilities|Casting|CastToBirdCharacterBlueprint (Game|Player|GetPlayerPawn 0)))
      (if (!= (Variables|/Game/Blueprints/BirdCharacterBlueprint.BirdCharacterBlueprint_C|GetMaxScore _asbirdcharacterblueprint_c_2) 0)
        (HUD|DrawText (Utilities|String|Append (Utilities|String|Append (Utilities|String|Append "SCORE: " (Utilities|String|ToString(Integer) (Variables|/Game/Blueprints/BirdCharacterBlueprint.BirdCharacterBlueprint_C|GetCurrentScore _asbirdcharacterblueprint_c_2))) " /") (Utilities|String|ToString(Integer) (Variables|/Game/Blueprints/BirdCharacterBlueprint.BirdCharacterBlueprint_C|GetMaxScore _asbirdcharacterblueprint_c_2))) _fontcolor _returnvalue_4 1e+01 _myfont 1.0 false)
        (else
          (HUD|DrawText (Utilities|String|Append "SCORE: " (Utilities|String|ToString(Integer) (Variables|/Game/Blueprints/BirdCharacterBlueprint.BirdCharacterBlueprint_C|GetCurrentScore _asbirdcharacterblueprint_c_2))) _fontcolor _returnvalue_4 1e+01 _myfont 1.0 false))))))

(event EventTick
  (params (DeltaSeconds :type Float%20%28single-precision%29))
  ;[1 1 1] Working Timer
  (if (== (Variables|Default|GetCountdown) 0.0)
    (Variables|Default|SetTimerNotCompleted false))
  (if (!= (Variables|Default|GetCountdown) 0.0)
    (Variables|Default|SetTimerActivated true)
    (if (Variables|Default|GetTimerActivated)
      (if (not (Variables|Default|GetTimerNotCompleted))
        (Variables|Default|SetTimerNotCompleted true)
        (Utilities|Time|SetTimerbyFunctionName 0 "TimerTicks" 1.0 (Variables|Default|GetTimerNotCompleted))))))

(fn ConstructionScript)

(fn TimerTicks
  (Variables|Default|SetCountdown (- (Variables|Default|GetCountdown) 1.0))
  (if (== (Variables|Default|GetCountdown) 0.0)
    (Variables|Default|SetTimerActivated false)
    (Variables|Default|SetTimerNotCompleted false)))