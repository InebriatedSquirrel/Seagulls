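; BoostRing is a boost pickup actor that pushes the player character along world +Y after anything overlaps its static mesh.
; Overlap sets a flag, and Tick uses it to start a looping 0.1-second Whoosh timer, with a second flag guarding against restarts.
; Whoosh repeatedly launches player 0 while counting Time down, printing debug text.
; At zero it resets Time and the boost flag but never clears the timer.
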(event OnComponentBeginOverlap(StaticMesh1)
  (params (OtherActor :type Actor%20Object%20Reference) (OtherComp :type Primitive%20Component%20Object%20Reference) (OtherBodyIndex :type Integer))
  (Variables|Default|SetBoosting true))

(event EventTick
  (params (DeltaSeconds :type Float%20%28single-precision%29))
  (if (Variables|Default|GetCaughtBoosting)
    (if (<= (Variables|Default|GetTime) 0.0)
      (Variables|Default|SetCaughtBoosting false))
    (elif (Variables|Default|GetBoosting)
      (Utilities|Time|SetTimerbyFunctionName 0 "Whoosh" 0.1 (Variables|Default|GetBoosting))
      (if (<= (Variables|Default|GetTime) 0.0)
        (Variables|Default|SetCaughtBoosting false)
        (else
          (Variables|Default|SetCaughtBoosting true))))))

(fn ConstructionScript)

(fn Whoosh
  (if (<= (Variables|Default|GetTime) 0.0)
    (Variables|Default|SetBoosting false)
    (Development|PrintString "WTF")
    (Variables|Default|SetTime 3.0)
    (else
      (Character|LaunchCharacter (Game|GetPlayerCharacter 0) "0,333.329987, 0" false false)
      (Variables|Default|SetTime (- (Variables|Default|GetTime) 0.1))
      (Development|PrintString (Utilities|String|ToString(Float) (Variables|Default|GetTime))))))