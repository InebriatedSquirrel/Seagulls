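; MissionLocation is an actor that shows mission text in the world and keeps turning to face the player's camera.
; The construction script applies the String and WorldSize variables to the MissionText component.
; Each Tick, it smoothly interpolates the whole actor's rotation toward the first player's camera, skipping the update while that camera sits at the world origin.
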(event EventTick
  (params (DeltaSeconds :type Float%20%28single-precision%29))
  (bind _returnvalue (Game|GetPlayerCameraManager 0))
  (bind _returnvalue_2 (Transformation|GetActorLocation _returnvalue))
  (if (!= _returnvalue_2 "0, 0, 0")
    (Transformation|SetActorRotation (Math|Interpolation|RInterpTo (Transformation|GetActorRotation) (Math|Rotator|FindLookatRotation (Transformation|GetActorLocation) _returnvalue_2) DeltaSeconds 5.0))))

(fn ConstructionScript
  (Rendering|Components|TextRender|SetText (Variables|Default|GetMissionText) (Variables|Default|GetSTring))
  (Rendering|Components|TextRender|SetWorldSize (Variables|Default|GetMissionText) (Variables|Default|GetWorldSize)))