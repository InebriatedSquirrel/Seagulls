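; Box of food prop Blueprint that varies its appearance by picking one of three textures at random.
; The Construction Script creates a dynamic material instance on the mesh's first material slot, then sets its texture parameter from a random integer switch.
; Because the roll happens during construction, the texture can change whenever the script reruns.
; The Event Graph holds an unconnected copy of the randomization that never runs.
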(fn ConstructionScript
  (Utilities|FlowControl|Sequence
    (:then_0
      ;[1 1 1] Make a dynamic material so the texture can change
      (bind _returnvalue (Rendering|Material|CreateDynamicMaterialInstance (Variables|Default|GetBoxOfFood) 0 0 :!class /Script/Engine.PrimitiveComponent))
      (Variables|Default|SetDynamicMaterial _returnvalue))
    (:then_1
      ;[1 1 1] Randomize the texture when placed
      (switch int (Math|Random|RandomIntegerinRange 0 2)
        (:Default
          (Rendering|Material|SetTextureParameterValue (Variables|Default|GetDynamicMaterial) "TextureParam" "/Game/Textures2/Texture_BoxofFood_1_T1.Texture_BoxofFood_1_T1" :!label _label))
        (:0
          (goto _label))
        (:1
          (Rendering|Material|SetTextureParameterValue (Variables|Default|GetDynamicMaterial) "TextureParam" "/Game/Textures2/Texture_BoxofFood_1_T2.Texture_BoxofFood_1_T2"))
        (:2
          (Rendering|Material|SetTextureParameterValue (Variables|Default|GetDynamicMaterial) "TextureParam" "/Game/Textures2/Texture_BoxofFood_1_T3.Texture_BoxofFood_1_T3"))))))