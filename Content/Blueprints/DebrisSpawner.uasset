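; DebrisSpawner is a spawner actor that periodically creates Debris actors at its own location.
; On the first Tick while Enabled, it sets a Start flag and starts a timer on SpawnDebris that fires every few seconds, looping according to Enabled.
; Each spawn copies the spawner's scale, randomizes rotation around a near-vertical pitch with slight yaw and roll, and does not force spawning when colliding.
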(event EventTick
  (params (DeltaSeconds :type Float%20%28single-precision%29))
  (if (Variables|Default|GetEnabled)
    (if (not (Variables|Default|GetStart))
      (Utilities|Time|SetTimerbyFunctionName 0 "SpawnDebris" 2.0 (Variables|Default|GetEnabled))
      (Variables|Default|SetStart true))))

(fn ConstructionScript)

(fn SpawnDebris
  (bind _returnvalue (Transformation|GetActorTransform))
  (bind (_location _rotation _scale) (Math|Transform|BreakTransform _returnvalue))
  (Game|SpawnActorfromClass "/Game/Blueprints/Debris.Debris_C" (Math|Transform|MakeTransform _location (Class|KismetMathLibrary|MakeRot (Math|Random|RandomFloatinRange 75.0 105.0) (Math|Random|RandomFloatinRange 0.0 3e+01) (Math|Random|RandomFloatinRange 0.0 3e+01)) _scale) false))