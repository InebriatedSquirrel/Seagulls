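; Collectible trophy pickup that destroys itself when any actor begins overlapping it.
; It then casts the player pawn, not the overlapping actor, to BirdCharacterBlueprint, increments TrophiesCollected and decrements TotalTrophies there.
; Debug PrintString messages announce the pickup and a count computed as TrophiesCollected plus one after the increment.
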(event EventActorBeginOverlap
  (params (OtherActor :type Actor%20Object%20Reference))
  (Actor|DestroyActor)
  (bind _asbirdcharacterblueprint_c (Utilities|Casting|CastToBirdCharacterBlueprint (Game|Player|GetPlayerPawn 0)))
  (Variables|/Game/Blueprints/BirdCharacterBlueprint.BirdCharacterBlueprint_C|SetTrophiesCollected _asbirdcharacterblueprint_c (+ (Variables|/Game/Blueprints/BirdCharacterBlueprint.BirdCharacterBlueprint_C|GetTrophiesCollected _asbirdcharacterblueprint_c) 1))
  (bind _asbirdcharacterblueprint_c_2 (Utilities|Casting|CastToBirdCharacterBlueprint (Game|Player|GetPlayerPawn 0)))
  (Variables|/Game/Blueprints/BirdCharacterBlueprint.BirdCharacterBlueprint_C|SetTotalTrophies _asbirdcharacterblueprint_c_2 (- (Variables|/Game/Blueprints/BirdCharacterBlueprint.BirdCharacterBlueprint_C|GetTotalTrophies _asbirdcharacterblueprint_c_2) 1))
  (Development|PrintString "Trophies!")
  (Development|PrintString (Utilities|String|ToString(Integer) (+ (Variables|/Game/Blueprints/BirdCharacterBlueprint.BirdCharacterBlueprint_C|GetTrophiesCollected _asbirdcharacterblueprint_c) 1)))
  (Development|PrintString "You now have:")
  (Development|PrintString "Added a trophy to your collection!"))

(fn ConstructionScript)