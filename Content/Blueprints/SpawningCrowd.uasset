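; SpawningCrowd is a crowd spawner that fills an area around its SpawnPoint with NPC actors when play begins.
; BeginPlay spawns Orphan actors at random points within RadiusOfSpawnArea, each with a random rotation, using NumberOfAdultMaleNPCs as the count.
; Similar loops for adult female, child female and male, and DestructibleCrab actors are disconnected and never run.
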(event EventBeginPlay
  (for _index (range 1 (Variables|Default|GetNumberOfAdultMaleNPCs))
    (Game|SpawnActorfromClass "/Game/Blueprints/Orphan.Orphan_C" (Math|Transform|MakeTransform (Class|NavigationSystem|GetRandomPointinRadius (Transformation|GetWorldLocation (Variables|Default|GetSpawnPoint)) (Variables|Default|GetRadiusOfSpawnArea)) (Math|Random|RandomRotator false)) false)))

(fn ConstructionScript)