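; Debug actor that visualizes a projectile's arc by drawing a short-lived debug sphere at its location every tick.
; BeginPlay speeds the actor up through custom time dilation, and Tick calls SpawnArcPoint to draw each point.
; Sphere green and alpha scale with elapsed lifespan, derived from the initial and remaining lifespan.
; A cooldown check for spacing the points is present but disconnected.
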(event EventTick
  (params (DeltaSeconds :type Float%20%28single-precision%29))
  (CallFunction|SpawnArcPoint))

(event EventBeginPlay
  (Variables|Default|SetCustomTimeDilation 5.0))

(fn ConstructionScript)

(fn SpawnArcPoint
  (bind _returnvalue (Actor|GetLifeSpan))
  (bind _initiallifespan (Variables|Actor|GetInitialLifeSpan))
  (bind _returnvalue_2 (- _returnvalue _initiallifespan))
  (bind _returnvalue_3 (* _returnvalue_2 -1.0))
  (Rendering|Debug|DrawDebugSphere (Transformation|GetActorLocation) 5.0 12 (Utilities|Struct|MakeLinearColor 0.0 _returnvalue_3 0.0 _returnvalue_3) 0.1))