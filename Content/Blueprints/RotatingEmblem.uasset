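; RotatingEmblem is an actor that displays a chosen emblem mesh and spins it continuously.
; The construction script assigns the DisplayedEmblem mesh to the Emblem component.
; Each tick adds RotateSpeed to the yaw of the Base component's world rotation, keeping pitch and roll, so the spin rate depends on frame rate rather than delta time.
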(event EventTick
  (params (DeltaSeconds :type Float%20%28single-precision%29))
  (bind _base (Variables|Default|GetBase))
  (bind _returnvalue (Transformation|GetWorldRotation _base))
  (bind (_pitch _yaw _roll) (Class|KismetMathLibrary|BreakRot _returnvalue))
  (Transformation|SetWorldRotation _base (Class|KismetMathLibrary|MakeRot _pitch (+ _yaw (Variables|Emblem|GetRotateSpeed)) _roll) false))

(fn ConstructionScript
  (Components|StaticMesh|SetStaticMesh (Variables|Default|GetEmblem) (Variables|Emblem|GetDisplayedEmblem)))