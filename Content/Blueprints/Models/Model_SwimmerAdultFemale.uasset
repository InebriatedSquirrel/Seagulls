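; Blueprint model of an adult female swimmer that randomizes its appearance in the Construction Script.
; One random roll shows either Hair1 or Hair2 and hides the other.
; A second, independent roll picks one of four paired looks, setting a hair color on both hair components and a matching material instance on the Child component.
; The rolls are unseeded, so the look can change whenever the script reruns.
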(fn ConstructionScript
  (bind _child (Variables|Default|GetChild))
  (bind _hair1 (Variables|Default|GetHair1))
  (bind _hair2 (Variables|Default|GetHair2))
  (bind _hair1_2 (Variables|Default|GetHair1))
  (Utilities|FlowControl|Sequence
    (:then_0
      ;[1 1 1] Randomize Which Hair Is Visible
      (switch int (Math|Random|RandomIntegerinRange 0 1)
        (:0
          (Utilities|FlowControl|Sequence
            (:then_0
              (Rendering|SetVisibility _hair1 true false))
            (:then_1
              (Rendering|SetVisibility _hair2 false false))))
        (:1
          (Utilities|FlowControl|Sequence
            (:then_0
              (Rendering|SetVisibility _hair1 false false))
            (:then_1
              (Rendering|SetVisibility _hair2 true false))))))
    (:then_1
      ;[1 1 1] Randomize Materials - Hair and Human
      (switch int (Math|Random|RandomIntegerinRange 0 3)
        (:Default
          (Utilities|FlowControl|Sequence :!label _label
            (:then_0
              (Rendering|Material|SetMaterial _hair1_2 0 "/Game/Materials2/Material_HumanHair_1_M1_Blonde.Material_HumanHair_1_M1_Blonde"))
            (:then_1
              (Rendering|Material|SetMaterial _child 0 "/Game/Materials2/Instances/Material_SwimmerAdultFemale_1_M1_Inst4.Material_SwimmerAdultFemale_1_M1_Inst4"))))
        (:0
          (Utilities|FlowControl|Sequence
            (:then_0
              (Rendering|Material|SetMaterial _hair1_2 0 "/Game/Materials2/Material_HumanHair_1_M1_Brown.Material_HumanHair_1_M1_Brown"))
            (:then_1
              (Rendering|Material|SetMaterial _child 0 "/Game/Materials2/Instances/Material_SwimmerAdultFemale_1_M1_Inst.Material_SwimmerAdultFemale_1_M1_Inst"))))
        (:1
          (Utilities|FlowControl|Sequence
            (:then_0
              (Rendering|Material|SetMaterial _hair1_2 0 "/Game/Materials2/Material_HumanHair_1_M1_Ginger.Material_HumanHair_1_M1_Ginger"))
            (:then_1
              (Rendering|Material|SetMaterial _child 0 "/Game/Materials2/Instances/Material_SwimmerAdultFemale_1_M1_Inst2.Material_SwimmerAdultFemale_1_M1_Inst2"))))
        (:2
          (Utilities|FlowControl|Sequence
            (:then_0
              (Rendering|Material|SetMaterial _hair1_2 0 "/Game/Materials2/Material_HumanHair_1_M1_Ginger.Material_HumanHair_1_M1_Ginger"))
            (:then_1
              (Rendering|Material|SetMaterial _child 0 "/Game/Materials2/Instances/Material_SwimmerAdultFemale_1_M1_Inst3.Material_SwimmerAdultFemale_1_M1_Inst3"))))
        (:3
          (goto _label))))))