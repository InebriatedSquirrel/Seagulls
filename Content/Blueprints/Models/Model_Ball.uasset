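; Ball model Blueprint that randomizes its look and size in the construction script.
; A random integer switch picks one of three material instances for the Ball component and sets its relative scale alongside it.
; Two variants are half size, while the third, which also serves as the default case, is full size.
; The roll is unseeded, so it can change whenever construction reruns.
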(fn ConstructionScript
  (bind _ball (Variables|Default|GetBall))
  ;[1 1 1] Randomize the texture and size when placed
  (switch int (Math|Random|RandomIntegerinRange 0 2)
    (:Default
      (Utilities|FlowControl|Sequence :!label _label
        (:then_0
          (Rendering|Material|SetMaterial _ball 0 "/Game/Materials2/Instances/Material_Ball_M1_Inst3.Material_Ball_M1_Inst3"))
        (:then_1
          (Transformation|SetRelativeScale3D _ball "1.000000,1.000000,1.000000"))))
    (:0
      (Utilities|FlowControl|Sequence
        (:then_0
          (Rendering|Material|SetMaterial _ball 0 "/Game/Materials2/Instances/Material_Ball_M1_Inst.Material_Ball_M1_Inst"))
        (:then_1
          (Transformation|SetRelativeScale3D _ball "0.500000,0.500000,0.500000"))))
    (:1
      (Utilities|FlowControl|Sequence
        (:then_0
          (Rendering|Material|SetMaterial _ball 0 "/Game/Materials2/Instances/Material_Ball_M1_Inst2.Material_Ball_M1_Inst2"))
        (:then_1
          (Transformation|SetRelativeScale3D _ball "0.500000,0.500000,0.500000"))))
    (:2
      (goto _label))))