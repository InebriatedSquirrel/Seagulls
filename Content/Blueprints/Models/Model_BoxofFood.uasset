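; Box of food prop Blueprint that varies its look each time it is constructed.
; The construction script picks a random integer and sets one of three material instances on the BoxOfFood component.
; An older EventGraph version that swaps the TextureParam texture on a dynamic material is left unconnected and never runs.
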(fn ConstructionScript
  (bind _boxoffood (Variables|Default|GetBoxOfFood))
  ;[1 1 1] Randomize the texture when placed
  (switch int (Math|Random|RandomIntegerinRange 0 2)
    (:Default
      (Rendering|Material|SetMaterial _boxoffood 0 "/Game/Materials2/Instances/Material_BoxofFood_1_M1_Inst.Material_BoxofFood_1_M1_Inst" :!label _label))
    (:0
      (goto _label))
    (:1
      (Rendering|Material|SetMaterial _boxoffood 0 "/Game/Materials2/Instances/Material_BoxofFood_1_M1_Inst2.Material_BoxofFood_1_M1_Inst2"))
    (:2
      (Rendering|Material|SetMaterial _boxoffood 0 "/Game/Materials2/Instances/Material_BoxofFood_1_M1_Inst3.Material_BoxofFood_1_M1_Inst3"))))