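; Game state for four-player local multiplayer that tracks each bird character's score and picks a winner.
; BeginPlay zeroes the four scores; AddScore copies Score from player pawns 0–3, stopping at the first failed BirdCharacterBlueprint cast.
; CheckWinner compares each score to the maximum in player order, so ties favour the lower number, then prints and stores the winner text.
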(event EventBeginPlay
  (CallFunction|InitializeScores))

(fn ConstructionScript)

(fn InitializeScores
  (Variables|Default|SetPlayerScore1 0)
  (Variables|Default|SetPlayerScore2 0)
  (Variables|Default|SetPlayerScore3 0)
  (Variables|Default|SetPlayerScore4 0))

(fn CheckWinner
  (bind _playerscore1 (Variables|Default|GetPlayerScore1))
  (bind _playerscore2 (Variables|Default|GetPlayerScore2))
  (bind _playerscore3 (Variables|Default|GetPlayerScore3))
  (bind _playerscore4 (Variables|Default|GetPlayerScore4))
  (bind _returnvalue (Math|Integer|Max(Integer) _playerscore1 _playerscore2 _playerscore3 _playerscore4))
  (if (== _returnvalue _playerscore1)
    (Variables|Default|SetWinner 1)
    (Development|PrintString (Utilities|String|Append "The Winner is Player " (Utilities|String|ToString(Integer) (Variables|Default|GetWinner))) :!label _label)
    (Variables|Default|SetWinnerString (Utilities|String|Append "The Winner is Player " (Utilities|String|ToString(Integer) (Variables|Default|GetWinner))))
    (elif (== _returnvalue _playerscore2)
      (Variables|Default|SetWinner 2)
      (goto _label)
      (elif (== _returnvalue _playerscore3)
        (Variables|Default|SetWinner 3)
        (goto _label)
        (elif (== _returnvalue _playerscore4)
          (Variables|Default|SetWinner 4)
          (goto _label))))))

(fn AddScore
  (bind _asbirdcharacterblueprint_c (Utilities|Casting|CastToBirdCharacterBlueprint (Game|Player|GetPlayerPawn 0)))
  (Variables|Default|SetPlayerScore1 (Variables|/Game/Blueprints/BirdCharacterBlueprint.BirdCharacterBlueprint_C|GetScore _asbirdcharacterblueprint_c))
  (bind _asbirdcharacterblueprint_c_2 (Utilities|Casting|CastToBirdCharacterBlueprint (Game|Player|GetPlayerPawn 1)))
  (Variables|Default|SetPlayerScore2 (Variables|/Game/Blueprints/BirdCharacterBlueprint.BirdCharacterBlueprint_C|GetScore _asbirdcharacterblueprint_c_2))
  (bind _asbirdcharacterblueprint_c_3 (Utilities|Casting|CastToBirdCharacterBlueprint (Game|Player|GetPlayerPawn 2)))
  (Variables|Default|SetPlayerScore3 (Variables|/Game/Blueprints/BirdCharacterBlueprint.BirdCharacterBlueprint_C|GetScore _asbirdcharacterblueprint_c_3))
  (bind _asbirdcharacterblueprint_c_4 (Utilities|Casting|CastToBirdCharacterBlueprint (Game|Player|GetPlayerPawn 3)))
  (Variables|Default|SetPlayerScore4 (Variables|/Game/Blueprints/BirdCharacterBlueprint.BirdCharacterBlueprint_C|GetScore _asbirdcharacterblueprint_c_4)))