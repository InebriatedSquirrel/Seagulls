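; A destructible cage actor that breaks apart after taking enough hits.
; While destruction is enabled, each Hit event subtracts Damage from Health.
; When Health equals exactly zero, radius damage with impulse at the hit location is applied to the Cage component.
; A short lifespan is then set so the actor removes itself.
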(event EventHit
  (params (MyComp :type Primitive%20Component%20Object%20Reference) (Other :type Actor%20Object%20Reference) (OtherComp :type Primitive%20Component%20Object%20Reference) (bSelfMoved :type Boolean) (HitLocation :type Vector :default "0, 0, 0") (HitNormal :type Vector :default "0, 0, 0") (NormalImpulse :type Vector :default "0, 0, 0") (Hit :type Hit%20Result%20Structure%20%28by%20ref%29))
  (if (Variables|Default|GetCanBeDestroyed)
    (Variables|Default|SetHealth (- (Variables|Default|GetHealth) (Variables|Default|GetDamage)))
    (Variables|Default|SetHealthAtZero (== (Variables|Default|GetHealth) 0))
    (if (Variables|Default|GetHealthAtZero)
      (Class|DestructibleComponent|ApplyRadiusDamage (Variables|Default|GetCage) 4.0 HitLocation 1e+02 1e+02 false)
      (Actor|SetLifeSpan 6.0))))

(fn ConstructionScript)