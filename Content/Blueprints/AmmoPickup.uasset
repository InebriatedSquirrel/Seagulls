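; Ammo pickup actor that grants the player's BirdCharacterBlueprint five ammo when its box trigger is overlapped.
; The overlap checks an Active flag and credits player pawn 0 regardless of which actor overlapped, then hides the mesh, disables collision and clears the flag.
; A timer calls Reset ten seconds later to restore visibility, collision and the flag, so the pickup respawns.
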(event OnComponentBeginOverlap(Box1)
  (params (OtherActor :type Actor%20Object%20Reference) (OtherComp :type Primitive%20Component%20Object%20Reference) (OtherBodyIndex :type Integer))
  (Development|PrintString "Hello")
  (if (Variables|Default|GetActive)
    (bind _asbirdcharacterblueprint_c (Utilities|Casting|CastToBirdCharacterBlueprint (Game|Player|GetPlayerPawn 0)))
    (Variables|/Game/Blueprints/BirdCharacterBlueprint.BirdCharacterBlueprint_C|SetAmmo _asbirdcharacterblueprint_c (+ (Variables|/Game/Blueprints/BirdCharacterBlueprint.BirdCharacterBlueprint_C|GetAmmo _asbirdcharacterblueprint_c) 5))
    (Rendering|SetVisibility (Variables|Default|GetStaticMesh1) false false)
    (Collision|SetActorEnableCollision false)
    (Variables|Default|SetActive false)
    (Utilities|Time|SetTimerbyFunctionName 0 "Reset" 1e+01)))

(event EventActorBeginOverlap
  (params (OtherActor :type Actor%20Object%20Reference)))

(fn ConstructionScript)

(fn Reset
  (Rendering|SetVisibility (Variables|Default|GetStaticMesh1) true false)
  (Collision|SetActorEnableCollision true)
  (Variables|Default|SetActive true))