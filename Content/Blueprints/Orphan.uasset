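; Orphan is an actor that serves as a scoring target for the bird character and resets to its starting spot.
; It records its location on BeginPlay and, on Hit, loops over all Projectile actors to test whether one struck it.
; A projectile hit spawns an explosion with sound, awards Points to the projectile's owning BirdCharacterBlueprint, then teleports the Orphan back.
; Contact with a Ground-tagged actor teleports it back without scoring.
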(event EventHit
  (params (MyComp :type Primitive%20Component%20Object%20Reference) (Other :type Actor%20Object%20Reference) (OtherComp :type Primitive%20Component%20Object%20Reference) (bSelfMoved :type Boolean) (HitLocation :type Vector :default "0, 0, 0") (HitNormal :type Vector :default "0, 0, 0") (NormalImpulse :type Vector :default "0, 0, 0") (Hit :type Hit%20Result%20Structure%20%28by%20ref%29))
  (bind _outactors (Actor|GetAllActorsOfClass "/Game/Blueprints/Projectile.Projectile_C"))
  (bind _array_element (Utilities|Array|ForEachLoopwithBreak _outactors)
    (:LoopBody
      _)
    (:Completed
      _))
  (if (== Other _array_element)
    (bind _returnvalue (Effects|SpawnEmitteratLocation "/Game/Particles/P_Explosion.P_Explosion" HitLocation))
    (Class|GameplayStatics|PlaySoundAttached "/Game/Audio/Explosion01.Explosion01" _returnvalue)
    (bind _asprojectile_c (Utilities|Casting|CastToProjectile))
    (bind _asbirdcharacterblueprint_c (Utilities|Casting|CastToBirdCharacterBlueprint (Variables|/Game/Blueprints/Projectile.Projectile_C|GetPojectileOwner _asprojectile_c)))
    (Variables|/Game/Blueprints/BirdCharacterBlueprint.BirdCharacterBlueprint_C|SetPointsAdded _asbirdcharacterblueprint_c (Variables|Default|GetPoints))
    (Default|AddPoints _asbirdcharacterblueprint_c)
    (Transformation|Teleport (Variables|Default|GetStartLocation) "0, 0, 0" :!label _label)
    (elif (Actor|ActorHasTag Other "Ground")
      (goto _label))))

(event EventBeginPlay
  (Utilities|FlowControl|DoOnce false
    (:Completed
      (Variables|Default|SetStartLocation (Transformation|GetActorLocation)))))

(fn ConstructionScript)