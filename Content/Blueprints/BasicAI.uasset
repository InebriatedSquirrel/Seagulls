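; BasicAI is a simple AI that wanders around a tether actor and flees when its Projectile hits it.
; A self-rescheduling IdleLoop timer moves it to random polar-offset points around the tether, with random stalls.
; A hit matching the Projectile variable shows debug text, stops wandering and moves it to the FleePoint actor, with no return to wandering.
; IdlePatrol offers an alternative random move but is not called here.
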(event Custom|IdleLoop
  ;[0.05769 0.05485 1] Wandering State
  (bind _newwanderpoint (CallFunction|FindWanderPoint))
  (AI|Navigation|SimpleMovetoLocation (Pawn|GetController) _newwanderpoint)
  (Utilities|Time|SetTimerbyFunctionName 0 "IdleLoop" (Math|Random|RandomFloatinRange (Variables|Default|GetWanderStallMin) (Variables|Default|GetWanderStallMax))))

(event EventBeginPlay
  (bind _tether (Variables|Default|GetTether))
  ;[0.05769 0.05485 1] Wandering State
  (Utilities|IsValid _tether
    (:Is%20Valid
      (Variables|Default|SetTetherPoint (Transformation|GetActorLocation _tether))
      (bind _newwanderpoint (CallFunction|FindWanderPoint))
      (AI|Navigation|SimpleMovetoLocation (Pawn|GetController) _newwanderpoint)
      (Utilities|Time|SetTimerbyFunctionName 0 "IdleLoop" (Math|Random|RandomFloatinRange (Variables|Default|GetWanderStallMin) (Variables|Default|GetWanderStallMax))))))

(event EventHit
  (params (MyComp :type Primitive%20Component%20Object%20Reference) (Other :type Actor%20Object%20Reference) (OtherComp :type Primitive%20Component%20Object%20Reference) (bSelfMoved :type Boolean) (HitLocation :type Vector :default "0, 0, 0") (HitNormal :type Vector :default "0, 0, 0") (NormalImpulse :type Vector :default "0, 0, 0") (Hit :type Hit%20Result%20Structure%20%28by%20ref%29))
  (bind _fleepoint (Variables|Default|GetFleePoint))
  (if (== Other "/Game/Blueprints/Projectile.Projectile")
    (Rendering|Debug|DrawDebugString HitLocation "HIT" 0 "(R=0.000000,G=0.000000,B=0.000000,A=1.000000)" 3.0)
    (Utilities|Time|ClearTimerbyFunctionName 0 "IdleLoop")
    (Utilities|IsValid _fleepoint
      (:Is%20Valid
        (Variables|Default|SetFleeSpot (Transformation|GetActorLocation _fleepoint))
        (AI|Navigation|SimpleMovetoLocation (Pawn|GetController) (Variables|Default|GetFleeSpot))))))

(fn ConstructionScript)

(fn IdlePatrol
  (AI|Navigation|SimpleMovetoLocation (Pawn|GetController) (Class|NavigationSystem|GetRandomPointinRadius (Transformation|GetActorLocation) 1e+03)))

(fn FindWanderPoint
  (bind _tetherpoint (Variables|Default|GetTetherPoint))
  (bind (_x _y _z) (Math|Vector|BreakVector _tetherpoint))
  (Variables|Default|SetRandMag (Math|Random|RandomFloatinRange 7e+01 (Variables|Default|GetWanderRadius)))
  (Variables|Default|SetRandAngle (Math|Random|RandomFloatinRange 0.0 359.0))
  (return (Math|Vector|MakeVector (+ (* (Variables|Default|GetRandMag) (Math|Trig|Cos(Degrees) (Variables|Default|GetRandAngle))) _x) (+ (* (Variables|Default|GetRandMag) (Math|Trig|Sin(Degrees) (Variables|Default|GetRandAngle))) _y) _z)))