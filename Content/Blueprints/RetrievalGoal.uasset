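; RetrievalGoal is a goal area that completes when its assigned GoalObject is inside it and the bird player is not grabbing it.
; Overlap events for GoalObject track whether it is inside and cache or clear the player's BirdCharacterBlueprint reference.
; Tick polls the bird's GrabbedObject until the object is released in the area, then prints a message and latches AccomplishedGoal.
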(event EventActorBeginOverlap
  (params (OtherActor :type Actor%20Object%20Reference))
  ;[0.1678 1 0.2058] Detect when the player and object enters the goal area
  (if (== OtherActor (Variables|Retrieval|GetGoalObject))
    (Variables|Default|SetGoalObjectInside true)
    (bind _asbirdcharacterblueprint_c (Utilities|Casting|CastToBirdCharacterBlueprint (Game|GetPlayerCharacter 0)))
    (Variables|Default|SetPlayerCharacter _asbirdcharacterblueprint_c)))

(event EventActorEndOverlap
  (params (OtherActor :type Actor%20Object%20Reference))
  ;[1 0.3097 0.3288] Detect when the player and object leaves the goal area
  (if (== OtherActor (Variables|Retrieval|GetGoalObject))
    (Variables|Default|SetGoalObjectInside false)
    (Variables|Default|SetPlayerCharacter 0)))

(event EventTick
  (params (DeltaSeconds :type Float%20%28single-precision%29))
  ;[0.1041 0.1513 1] If the goal hasn't been accomplished, and
  (if (not (Variables|Default|GetAccomplishedGoal))
    (if (Variables|Default|GetGoalObjectInside)
      ;[0.1041 0.1513 1] Make sure that the target object is not currently grabbed, if not, goal accomplished
      (bind _asbirdcharacterblueprint_c (Utilities|Casting|CastToBirdCharacterBlueprint (Variables|Default|GetPlayerCharacter)))
      (if (not (== (Variables|Retrieval|GetGoalObject) (Variables|/Game/Blueprints/BirdCharacterBlueprint.BirdCharacterBlueprint_C|GetGrabbedObject _asbirdcharacterblueprint_c)))
        (Development|PrintString "Goal Accomplished")
        (Variables|Default|SetGoalObjectInside false)
        (Variables|Default|SetAccomplishedGoal true)))))

(fn ConstructionScript)