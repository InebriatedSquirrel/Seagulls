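; Swimming adult female NPC that wanders until hit by a projectile (bird poop), then runs away.
; A self-restarting timer moves it to random points around its spawn-time tether, pausing randomly between moves.
; On hit, it matches the other actor against all Projectile actors, stops wandering and, given a valid FleePoint, speeds toward it.
; The first such hit flags it as pooped on only when the player bird's level number is 2.3.
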(event Custom|IdleLoop
  ;[0.05769 0.05485 1] Wandering State
  (bind _newwanderpoint (CallFunction|FindWanderPoint))
  (AI|Navigation|SimpleMovetoLocation (Pawn|GetController) _newwanderpoint)
  (Utilities|Time|SetTimerbyFunctionName 0 "IdleLoop" (Math|Random|RandomFloatinRange (Variables|Default|GetWanderStallMin) (Variables|Default|GetWanderStallMax))))

(event EventBeginPlay
  ;[0.05769 0.05485 1] Wandering State
  (Variables|Default|SetTetherPoint (Transformation|GetActorLocation (Pawn|GetController)))
  (bind _newwanderpoint (CallFunction|FindWanderPoint))
  (AI|Navigation|SimpleMovetoLocation (Pawn|GetController) _newwanderpoint)
  (Utilities|Time|SetTimerbyFunctionName 0 "IdleLoop" (Math|Random|RandomFloatinRange (Variables|Default|GetWanderStallMin) (Variables|Default|GetWanderStallMax))))

(event EventHit
  (params (MyComp :type Primitive%20Component%20Object%20Reference) (Other :type Actor%20Object%20Reference) (OtherComp :type Primitive%20Component%20Object%20Reference) (bSelfMoved :type Boolean) (HitLocation :type Vector :default "0, 0, 0") (HitNormal :type Vector :default "0, 0, 0") (NormalImpulse :type Vector :default "0, 0, 0") (Hit :type Hit%20Result%20Structure%20%28by%20ref%29))
  (bind _fleepoint (Variables|Default|GetFleePoint))
  ;[1 1 1] What happens when they get shit on
  (bind _outactors (Actor|GetAllActorsOfClass "/Game/Blueprints/Projectile.Projectile_C"))
  (bind _array_element (Utilities|Array|ForEachLoopwithBreak _outactors)
    (:LoopBody
      _)
    (:Completed
      _))
  (if (== Other _array_element)
    (Utilities|Time|ClearTimerbyFunctionName 0 "IdleLoop")
    (Utilities|IsValid _fleepoint
      (:Is%20Valid
        (Variables|Default|SetFleeSpot (Transformation|GetActorLocation _fleepoint))
        (Variables|/Script/Engine.CharacterMovementComponent|SetMaxWalkSpeed (Variables|Character|GetCharacterMovement) 6e+02)
        (AI|Navigation|SimpleMovetoLocation (Pawn|GetController) (Variables|Default|GetFleeSpot))
        (if (not (Variables|Default|GetInitialHit))
          (bind _asbirdcharacterblueprint_c (Utilities|Casting|CastToBirdCharacterBlueprint (Game|Player|GetPlayerPawn 0)))
          (if (== (Variables|/Game/Blueprints/BirdCharacterBlueprint.BirdCharacterBlueprint_C|GetCurrentLevelNumber _asbirdcharacterblueprint_c) 2.3)
            (Variables|Default|SetHasBeenPoopedOn true)
            (Variables|Default|SetInitialHit true)))))))

(fn ConstructionScript)

(fn FindWanderPoint
  (bind _tetherpoint (Variables|Default|GetTetherPoint))
  (bind (_x _y _z) (Math|Vector|BreakVector _tetherpoint))
  (Variables|Default|SetRandMag (Math|Random|RandomFloatinRange 7e+01 (Variables|Default|GetWanderRadius)))
  (Variables|Default|SetRandAngle (Math|Random|RandomFloatinRange 0.0 359.0))
  (return (Math|Vector|MakeVector (+ (* (Variables|Default|GetRandMag) (Math|Trig|Cos(Degrees) (Variables|Default|GetRandAngle))) _x) (+ (* (Variables|Default|GetRandMag) (Math|Trig|Sin(Degrees) (Variables|Default|GetRandAngle))) _y) _z)))