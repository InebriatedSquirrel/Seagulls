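; Adult female pedestrian NPC that wanders, then flees when hit by the player bird's droppings.
; IdleLoop moves it to the bird's CurrentLocation on a random stall timer, which Tick re-arms after a delay while the bird is within SafeDistance.
; A hit matching a Projectile actor speeds it toward FleePoint.
; Timer clears target "ChildFemale_All" rather than IdleLoop, so they do not cancel the wander loop.
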(event Custom|IdleLoop
  ;[0.05769 0.05485 1] Wandering State
  (bind _newwanderpoint (CallFunction|FindWanderPoint))
  (AI|Navigation|SimpleMovetoLocation (Pawn|GetController) _newwanderpoint)
  (Utilities|Time|SetTimerbyFunctionName 0 "IdleLoop" (Math|Random|RandomFloatinRange (Variables|Default|GetWanderStallMin) (Variables|Default|GetWanderStallMax))))

(event EventBeginPlay
  ;[0.05769 0.05485 1] Wandering State
  (bind _newwanderpoint (CallFunction|FindWanderPoint))
  (AI|Navigation|SimpleMovetoLocation (Pawn|GetController) _newwanderpoint)
  (Utilities|Time|SetTimerbyFunctionName 0 "IdleLoop" (Math|Random|RandomFloatinRange (Variables|Default|GetWanderStallMin) (Variables|Default|GetWanderStallMax))))

(event EventHit
  (params (MyComp :type Primitive%20Component%20Object%20Reference) (Other :type Actor%20Object%20Reference) (OtherComp :type Primitive%20Component%20Object%20Reference) (bSelfMoved :type Boolean) (HitLocation :type Vector :default "0, 0, 0") (HitNormal :type Vector :default "0, 0, 0") (NormalImpulse :type Vector :default "0, 0, 0") (Hit :type Hit%20Result%20Structure%20%28by%20ref%29))
  (bind _fleepoint (Variables|Default|GetFleePoint))
  ;[1 1 1] What happens when they get shit on
  (bind _outactors (Actor|GetAllActorsOfClass "/Game/Blueprints/Projectile.Projectile_C"))
  (bind _array_element (Utilities|Array|ForEachLoopwithBreak _outactors)
    (:LoopBody
      _)
    (:Completed
      _))
  (if (== Other _array_element)
    (Rendering|Debug|DrawDebugString HitLocation "HIT" 0 "(R=0.000000,G=0.000000,B=0.000000,A=1.000000)" 3.0)
    (Utilities|Time|ClearTimerbyFunctionName 0 "ChildFemale_All")
    (Utilities|IsValid _fleepoint
      (:Is%20Valid
        (Variables|Default|SetFleeSpot (Transformation|GetActorLocation _fleepoint))
        (Variables|/Script/Engine.CharacterMovementComponent|SetMaxWalkSpeed (Variables|Character|GetCharacterMovement) 6e+02)
        (AI|Navigation|SimpleMovetoLocation (Pawn|GetController) (Variables|Default|GetFleeSpot))))))

(event EventTick
  (params (DeltaSeconds :type Float%20%28single-precision%29))
  (bind _asbirdcharacterblueprint_c (Utilities|Casting|CastToBirdCharacterBlueprint (Game|GetPlayerCharacter 0)))
  (bind _returnvalue (Transformation|GetDistanceTo _asbirdcharacterblueprint_c))
  (Variables|Default|SetDistanceApart _returnvalue)
  (if (> (Variables|Default|GetDistanceApart) (Variables|Default|GetSafeDistance))
    (Utilities|Time|ClearTimerbyFunctionName 0 "ChildFemale_All")
    (else
      (Utilities|FlowControl|Delay 1.0)
      ;[0.05769 0.05485 1] Wandering State
      (Utilities|Time|SetTimerbyFunctionName 0 "IdleLoop" (Math|Random|RandomFloatinRange (Variables|Default|GetWanderStallMin) (Variables|Default|GetWanderStallMax))))))

(fn ConstructionScript)

(fn FindWanderPoint
  (bind _asbirdcharacterblueprint_c (Utilities|Casting|CastToBirdCharacterBlueprint (Game|GetPlayerCharacter 0)))
  (return (Variables|/Game/Blueprints/BirdCharacterBlueprint.BirdCharacterBlueprint_C|GetCurrentLocation _asbirdcharacterblueprint_c)))