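; Player seagull character that poops projectiles, grabs objects and tracks mission progress and score.
; Firing spends ammo that a looping timer recharges.
; Tick drives a physics handle, sphere-tracing below the grab origin for "Grab"-tagged objects, and mirrors ignored move input to block actions during cutscenes, which are skippable by cancelling Matinee.
; BeginPlay maps the level number to mission text, and AddPoints updates score text and game state.
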(event Custom|HasFlapped_Event
  ;[1 1 1] Flap Sound- needs work
)

(event Custom|AddPoints
  (bind _score (CallFunction|GetScore))
  (Rendering|Components|TextRender|SetText (Variables|Default|GetText1.0) (Utilities|String|ToString(Integer) _score))
  (bind _asmultiplayergamestate_c (Utilities|Casting|CastToMultiplayerGameState (Game|GetGameState)))
  (Default|AddScore _asmultiplayergamestate_c))

(event EventBeginPlay
  ;[1 1 1] Recharge Ammo
  (Utilities|Time|SetTimerbyFunctionName 0 "Recharge" 5.0 true)
  (CallFunction|LevelNumberSelection)
  ;[1 1 1] Flap Sound- needs work
  (EventDispatchers|BindEventtoHasFlapped (delegate Custom|HasFlapped_Event)))

(event EventTick
  (params (DeltaSeconds :type Float%20%28single-precision%29))
  (bind _graborigin (Variables|Default|GetGrabOrigin))
  (bind _returnvalue (Transformation|GetWorldLocation _graborigin))
  (bind (_x _y _z) (Math|Vector|BreakVector _returnvalue))
  (bind (_x_2 _y_2 _z_2) (Math|Vector|BreakVector _returnvalue))
  ;[1 1 1] Disable input toggle for cutscenes
  (bind _asplayercontroller (Utilities|Casting|CastToPlayerController (Pawn|GetController)))
  (Variables|Default|SetInputDisabled (Class|PlayerController|IsMoveInputIgnored _asplayercontroller))
  ;[0.1041 0.1513 1] Update Position of Handle
  (Variables|Default|SetCurrentLocation (Transformation|GetActorLocation))
  (Physics|Components|PhysicsHandle|SetTargetLocation (Variables|Default|GetPhysicsHandle) (Transformation|GetWorldLocation (Variables|Default|GetGrabOrigin)))
  (if (Variables|Default|GetPhysicsHandleActive)
    (if (Variables|Default|GetObjectIsGrabbed)
      ;[1 0.3097 0.3288] Release the Physics Component
      (Physics|Components|PhysicsHandle|ReleaseComponent (Variables|Default|GetPhysicsHandle))
      (Variables|Grabbing|SetGrabbedObject 0)
      (else
        ;[0.1041 0.1513 1] Cast a check for a Physics Object
        (bind (_outhit _returnvalue_2) (Collision|SphereTraceForObjects (Math|Vector|MakeVector _x _y (- _z 0.0)) (Math|Vector|MakeVector _x_2 _y_2 (- _z_2 5e+01)) 3e+01 (Utilities|Array|MakeArray (Variables|Default|GetGrabObjectType)) false 0 "ForDuration"))
        ;[0.1678 1 0.2058] Attach the Physics Object
        (if _returnvalue_2
          (if (Actor|ActorHasTag (.HitActor (Collision|BreakHitResult _outhit)) "Grab")
            (Variables|Grabbing|SetGrabbedObject (.HitActor (Collision|BreakHitResult _outhit)))
            (Transformation|SetActorTransform (.HitActor (Collision|BreakHitResult _outhit)) (Transformation|GetWorldTransform (Variables|Default|GetGrabOrigin)) true)
            (Collision|SetCollisionResponsetoChannel (.HitComponent (Collision|BreakHitResult _outhit)) "ECC_Pawn" "ECR_Ignore")
            (Collision|SetCollisionResponsetoChannel (.HitComponent (Collision|BreakHitResult _outhit)) "ECC_Camera" "ECR_Ignore")
            (Class|PhysicsHandleComponent|GrabComponent (Variables|Default|GetPhysicsHandle) (.HitComponent (Collision|BreakHitResult _outhit)) (.HitBoneName (Collision|BreakHitResult _outhit)) (.Location (Collision|BreakHitResult _outhit)) true)
            (Variables|Default|SetPhysicsHandleActive false)
            (Variables|Default|SetObjectIsGrabbed true)
            ;[1 1 1] Grab Sound
            (Class|GameplayStatics|PlaySoundAttached "/Game/Audio/seagullGrabFX.seagullGrabFX" (Variables|Default|GetGrabSoundFX))))))))

(event EventFlapped
  ;[1 1 1] Flap Sound- needs work
  (Class|GameplayStatics|PlaySoundAttached "/Game/Audio/seagullFlapFX.seagullFlapFX" (Variables|Default|GetFlapSoundFX))
  (Default|CallHasFlapped))

(event EventHit
  (params (MyComp :type Primitive%20Component%20Object%20Reference) (Other :type Actor%20Object%20Reference) (OtherComp :type Primitive%20Component%20Object%20Reference) (bSelfMoved :type Boolean) (HitLocation :type Vector :default "0, 0, 0") (HitNormal :type Vector :default "0, 0, 0") (NormalImpulse :type Vector :default "0, 0, 0") (Hit :type Hit%20Result%20Structure%20%28by%20ref%29))
  ;[1 1 1] Collision Sound - needs work
  (if (not (Actor|ActorHasTag Other "Ground"))
    (Class|GameplayStatics|PlaySoundAttached "/Game/Audio/seagullCollisionFX.seagullCollisionFX" (Variables|Default|GetCollisionSoundFX))))

(event Input|ActionEvents|InputActionGrab
  ;[0.1041 0.1513 1] Handle Input toggling
  (:Pressed
    (if (not (Variables|Default|GetInputDisabled))
      (Variables|Default|SetPhysicsHandleActive true)
      (if (Variables|Default|GetObjectIsGrabbed)
        (Utilities|FlowControl|Delay 1.0)
        (Variables|Default|SetObjectIsGrabbed false)
        (Collision|SetCollisionResponsetoChannel (.HitComponent (Collision|BreakHitResult (stale EventTick _outhit))) "ECC_Pawn" "ECR_Block"))))
  (:Released
    (Variables|Default|SetPhysicsHandleActive false)))

(event Input|ActionEvents|InputActionExit
  ;[1 1 1] Exit to menu or exit cutscene
  (:Pressed
    (if (Variables|Default|GetInputDisabled)
      ;[1 1 1] Skip cutscenes
      (bind _outactors (Actor|GetAllActorsOfClass "/Script/Engine.MatineeActor"))
      (for _array_element _outactors
        (bind _asmatineeactor (Utilities|Casting|CastToMatineeActor _array_element))
        (Development|ExecuteConsoleCommand "CANCELMATINEE"))
      (else
        (Game|OpenLevel(byName) "Main_Menu")))))

(event Input|ActionEvents|InputActionFireProjectile
  ;[1 1 1] Firing a Projectile (poop)
  (:Pressed
    (if (not (Variables|Default|GetInputDisabled))
      (Variables|Projectile|SetCharacterVelocity (Transformation|GetVelocity))
      ;[1 1 1] Ammo Inventory
      (if (>= (Variables|Default|GetAmmo) (Variables|Default|GetPlusOne))
        (Variables|Default|SetAmmo (- (Variables|Default|GetAmmo) (Variables|Default|GetPlusOne)))
        ;[1 1 1] Poop Sound
        (Class|GameplayStatics|PlaySoundAttached "/Game/Audio/seagullPooFX.seagullPooFX" (Variables|Default|GetPooSoundFX))
        (bind _returnvalue (Game|SpawnActorfromClass :Class "/Game/Blueprints/Projectile.Projectile_C" :SpawnTransform (Math|Transform|MakeTransform (+ (Transformation|GetActorLocation) (* (Transformation|GetActorUpVector) -4e+01)) (Pawn|GetControlRotation :!class /Script/Engine.Pawn))))
        (Collision|SetCollisionResponsetoChannel (Variables|/Game/Blueprints/Projectile.Projectile_C|GetSphere1 _returnvalue) "ECC_Pawn" "ECR_Ignore")
        (Collision|SetCollisionResponsetoChannel (Variables|/Game/Blueprints/Projectile.Projectile_C|GetSphere1 _returnvalue) "ECC_Camera" "ECR_Ignore")))))

(event Input|KeyboardEvents|T
  ;[1 1 1] Level cheat
  (:Pressed
    (Variables|Default|SetCurrentLevelNumber 6.4)))

(event Input|KeyboardEvents|Enter
  ;[1 1 1] Skip cutscenes
  (:Pressed
    (bind _outactors (Actor|GetAllActorsOfClass "/Script/Engine.MatineeActor"))
    (for _array_element _outactors
      (bind _asmatineeactor (Utilities|Casting|CastToMatineeActor _array_element))
      (Development|ExecuteConsoleCommand "CANCELMATINEE"))))

(fn ConstructionScript)

(fn Recharge
  (if (< (Variables|Default|GetAmmo) (Variables|Default|GetPlusFive))
    (Variables|Default|SetAmmo (+ (Variables|Default|GetAmmo) (Variables|Default|GetPlusOne)))))

(fn LevelNumberSelection
  (if (== 1.0 (Variables|Default|GetCurrentLevelNumber))
    (Variables|Default|SetMissionText "Walk through the ring")
    (else
      ;[1 1 1] 1.1 FLYING
      (if (== 1.1 (Variables|Default|GetCurrentLevelNumber))
        (Variables|Default|SetMissionText "Fly through the rings")
        (else
          ;[1 1 1] 1.2 RETURN TO NEST
          (if (== 1.2 (Variables|Default|GetCurrentLevelNumber))
            (Variables|Default|SetMissionText "Fly back to the nest")
            (else
              ;[1 1 1] 2.0 FIND SAL
              (if (== 2.0 (Variables|Default|GetCurrentLevelNumber))
                (Variables|Default|SetMissionText "Find Sal at the lighthouse")
                (else
                  ;[1 1 1] 2.1 COLLECTION (P1)
                  (if (== 2.1 (Variables|Default|GetCurrentLevelNumber))
                    (Variables|Default|SetMissionText "Find bags of Cheetos near the boardwalk for Sal")
                    (else
                      ;[1 1 1] 2.1 COLLECTION (P2)
                      (if (== 2.12 (Variables|Default|GetCurrentLevelNumber))
                        (Variables|Default|SetMissionText "Find pieces of candy near the pier for Sal")
                        (else
                          ;[1 1 1] 2.1 COLLECTION (P3)
                          (if (== 2.13 (Variables|Default|GetCurrentLevelNumber))
                            (Variables|Default|SetMissionText "Find some ice cream near the rides for Sal ")
                            (else
                              ;[1 1 1] 2.15 FIND SID
                              (if (== 2.15 (Variables|Default|GetCurrentLevelNumber))
                                (Variables|Default|SetMissionText "Find Sid by the pier")
                                (else
                                  ;[1 1 1] 2.2 DESTRUCTION
                                  (if (== 2.2 (Variables|Default|GetCurrentLevelNumber))
                                    (Variables|Default|SetMissionText "Destroy 10 crabs on the beach for Sid")
                                    (else
                                      ;[1 1 1] 2.3 DESTRUCTION (KEG PARTY)
                                      (if (== 2.3 (Variables|Default|GetCurrentLevelNumber))
                                        (Variables|Default|SetMissionText "Poop on people near the keg to break up the party for Sid")
                                        (else
                                          ;[1 1 1] 3.0 FIND SPEEDY
                                          (if (== 3.0 (Variables|Default|GetCurrentLevelNumber))
                                            (Variables|Default|SetMissionText "Find Speedy near the volley ball nets")
                                            (else
                                              ;[1 1 1] 3.1 GLIDING
                                              (if (== (Variables|Default|GetCurrentLevelNumber) 3.1)
                                                (Variables|Default|SetMissionText "Glide through the rings to get to the city")
                                                (else
                                                  ;[1 1 1] 4.0 LOCATE SARAH
                                                  (if (== 4.0 (Variables|Default|GetCurrentLevelNumber))
                                                    (Variables|Default|SetMissionText "Find Sarah in the city")
                                                    (else
                                                      ;[1 1 1] 5.1 SCAVENGER HUNT
                                                      (if (== 5.1 (Variables|Default|GetCurrentLevelNumber))
                                                        (Variables|Default|SetMissionText "Find a bungie cord, satellite dish, cell phone, and the sword.")
                                                        (else
                                                          ;[1 1 1] 6.1 DESTRUCTION OF MOUNTAIN
                                                          (if (== 6.1 (Variables|Default|GetCurrentLevelNumber))
                                                            (Variables|Default|SetMissionText "Destroy 10 pigeon totems and free Mama Bird")
                                                            (else
                                                              ;[1 1 1] 7.0 THE ESCAPE (RINGS)
                                                              (if (== 6.1 (Variables|Default|GetCurrentLevelNumber))
                                                                (Variables|Default|SetMissionText "Make your escape through the rings!")))))))))))))))))))))))))))))))))

(fn GetScore
  (Variables|Default|SetScore (+ (Variables|Default|GetScore) (Variables|Default|GetPointsAdded)))
  (return (Variables|Default|GetScore)))